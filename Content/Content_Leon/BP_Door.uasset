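; BP_Door is a door actor that moves vertically when interacted with, then stops blocking.
; BeginPlay turns TargetHeight from an offset into an absolute Z based on the starting height.
; Interact plays a timeline that lerps from the actor's current location toward that height, compounding each update.
; A second timeline then drives the cube material's Time parameter, and collision is disabled when it finishes.
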(event EventInteract
  (params (Instigator :type Pawn%20Object%20Reference))
  (bind _returnvalue (Transformation|GetActorLocation))
  (bind _lerp_0_1 (Timeline|LerpTimeline Play)
    (:Update
      (Transformation|SetActorLocation (Math|Vector|Lerp(Vector) (Transformation|GetActorLocation) (Math|Vector|MakeVector (.x _returnvalue) (.y _returnvalue) (Variables|Default|GetTargetHeight)) _lerp_0_1) false false))
    (:Finished
      (bind _newtrack_0 (Timeline|Timeline_0 Play)
        (:Update
          (Rendering|Material|SetScalarParameterValueonMaterials (Variables|Default|GetCube) "Time" _newtrack_0))
        (:Finished
          (Collision|SetCollisionEnabled (Variables|Default|GetCube) "NoCollision"))))))

(event EventBeginPlay
  (bind _output_get (Variables|Default|SetInitialHeight (.z (Transformation|GetActorLocation))))
  (Variables|Default|SetTargetHeight (+ _output_get (Variables|Default|GetTargetHeight))))

(fn ConstructionScript)