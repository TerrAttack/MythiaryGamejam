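; BP_Torch is a toggleable torch that sets overlapping vines alight and triggers game over.
; Interact switches its Niagara flame and active state, which is also applied on BeginPlay.
; It binds to the game mode's other-actors action event; Action collects overlapping curved and straight vines.
; If lit with vines collected, it spawns fire particles above each, then loads GameOver through the game mode after a delay.
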(event Custom|Event%20Action
  (bind _overlapcollider (Variables|Default|GetOverlapCollider))
  (bind _overlapcollider_2 (Variables|Default|GetOverlapCollider))
  (bind _overlappingactors (Variables|Default|GetOverlappingActors))
  (bind _overlappingactors_2 (Collision|GetOverlappingActors _overlapcollider "/Game/Content_Tjaard/BP_VineStraight.BP_VineStraight_C" :!class /Script/Engine.PrimitiveComponent))
  (bind _overlappingactors_3 (Collision|GetOverlappingActors _overlapcollider_2 "/Game/Content_Tjaard/BP_VineCurve.BP_VineCurve_C" :!class /Script/Engine.PrimitiveComponent))
  (Utilities|FlowControl|Sequence
    (:then_0
      ;[1 1 1] Fill OverlappingActors Array
      (if (Utilities|Array|IsNotEmpty _overlappingactors_3)
        (for _array_element _overlappingactors_3
          (Utilities|Array|Add (Variables|Default|GetOverlappingActors) _array_element))))
    (:then_1
      (if (Utilities|Array|IsNotEmpty _overlappingactors_2)
        (for _array_element_2 _overlappingactors_2
          (Utilities|Array|Add (Variables|Default|GetOverlappingActors) _array_element_2))))
    (:then_2
      ;[1 1 1] Spawn Fire Particles At Overlapped Actors
      (if (and (Utilities|Array|IsNotEmpty _overlappingactors) (Variables|Default|GetbIsTorchActive))
        (for _array_element_3 _overlappingactors
          (Niagara|SpawnSystematLocation "/Game/Import_Leon/Torch/NewNiagaraSystem.NewNiagaraSystem" (Math|Vector|MakeVector (.x (Transformation|GetActorLocation _array_element_3)) (.y (Transformation|GetActorLocation _array_element_3)) (+ (.z (Transformation|GetActorLocation _array_element_3)) 1e+01))))
        ;[1 1 1] Go To Gameover Level
        (Utilities|FlowControl|Delay 3.0)
        (bind _aspgame_mode_base (Utilities|Casting|CastToPGameModeBase (Game|GetGameMode)))
        (Class|PGameModeBase|LoadLevel _aspgame_mode_base "GameOver")))))

(event EventBeginPlay
  ;[1 1 1] Set Torch State
  (Utilities|FlowControl|Sequence
    (:then_0
      (if (Variables|Default|GetbIsTorchActive)
        (CallFunction|ActivateTorch)
        (else
          (CallFunction|DeactivateTorch))))
    (:then_1
      ;[1 1 1] Bind OnAction Event
      (bind _aspgame_mode_base (Utilities|Casting|CastToPGameModeBase (Game|GetGameMode)))
      (EventDispatchers|BindEventtoOnOtherActorsAction _aspgame_mode_base (delegate Custom|Event%20Action)))))

(event EventInteract
  (params (Instigator :type Pawn%20Object%20Reference))
  ;[1 1 1] Toggle Torch
  (if (not (Variables|Default|GetbIsTorchActive))
    (CallFunction|ActivateTorch)
    (else
      (CallFunction|DeactivateTorch))))

(fn ConstructionScript)

(fn ActivateTorch
  (Components|Activation|SetActive (Variables|Default|GetNiagara) true false)
  (Variables|Default|SetbIsTorchActive true))

(fn DeactivateTorch
  (Components|Activation|SetActive (Variables|Default|GetNiagara) false false)
  (Variables|Default|SetbIsTorchActive false))